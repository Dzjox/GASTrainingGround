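; Gameplay ability for the first attack of a sword combo, which commits on activation and plays a montage.
; While the montage runs, it listens for gameplay events marking the opening and closing of the combo window.
; The open event adds a non-replicated loose combo-window tag to the avatar; the close event removes it and ends the ability.
; Montage completion also ends the ability, without removing the tag.
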(event `self.K2_ActivateAbility`
  (`self.K2_CommitAbility`)
  (`AbilityTask_PlayMontageAndWait.CreatePlayMontageAndWaitProxy` "None" (`self.Montage to Play`)
    (:`then`
      (`AbilityTask_WaitGameplayEvent.WaitGameplayEvent` (struct :`TagName` "Event.ComboWindowOpen") null
        (:`then`
          (`AbilityTask_WaitGameplayEvent.WaitGameplayEvent` (struct :`TagName` "Event.ComboWindowClose") null
            (:`EventReceived`
              (`AbilitySystemBlueprintLibrary.RemoveLooseGameplayTags` (`self.GetAvatarActorFromActorInfo`) (`self.ComboWindowOpenTag`))
              (`self.K2_EndAbility`))))
        (:`EventReceived`
          (`AbilitySystemBlueprintLibrary.AddLooseGameplayTags` (`self.GetAvatarActorFromActorInfo`) (`self.ComboWindowOpenTag`)))))
    (:`OnCompleted`
      (`self.K2_EndAbility`))))