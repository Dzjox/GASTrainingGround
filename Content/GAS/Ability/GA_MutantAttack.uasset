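; Gameplay ability for the mutant's attack, dealing armor-aware damage through GAS.
; On successful commit it plays the attack montage and listens for the Event.MutantAttack gameplay event.
; The event applies GE_DamageWithArmor to the payload's target, passing the Damage variable as a SetByCaller magnitude.
; The ability ends when the montage completes, blends out or is interrupted or cancelled; a failed commit has no EndAbility path.
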(event `self.K2_ActivateAbility`
  (bind _returnvalue (`self.K2_CommitAbility`))
  (if _returnvalue
    (`AbilityTask_PlayMontageAndWait.CreatePlayMontageAndWaitProxy` "None" "/Game/MIxamo/Monster/AM_MutantAttack.AM_MutantAttack"
      (:`then`
        (bind (_asynctaskproxy _payload) (`AbilityTask_WaitGameplayEvent.WaitGameplayEvent` (struct :`TagName` "Event.MutantAttack") null)
          (:`EventReceived`
            (bind _returnvalue_2 (`AbilitySystemBlueprintLibrary.AssignTagSetByCallerMagnitude` (`self.MakeOutgoingGameplayEffectSpec` "/Game/GAS/Effects/GE_DamageWithArmor.GE_DamageWithArmor_C") (struct :`TagName` "Data.Damage") (`self.Damage`)))
            (`AbilitySystemComponent.BP_ApplyGameplayEffectSpecToTarget` (`AbilitySystemBlueprintLibrary.GetAbilitySystemComponent` (`self.GetAvatarActorFromActorInfo`)) _returnvalue_2 (`AbilitySystemBlueprintLibrary.GetAbilitySystemComponent` (`.Target` (break `GameplayEventData` _payload)))))))
      (:`OnCompleted`
        (`self.K2_EndAbility` :!label _label))
      (:`OnBlendOut`
        (goto _label))
      (:`OnInterrupted`
        (goto _label))
      (:`OnCancelled`
        (goto _label)))))