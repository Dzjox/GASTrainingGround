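; Gameplay ability for the second step of a sword combo, which commits and plays an attack montage.
; While it plays, it listens for combo window gameplay events: opening swaps the previous step's window tag for its own on the avatar.
; Closing removes that tag and ends the ability, as does montage completion, which leaves the tag untouched.
; The tags are loose and non-replicated.
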(event `self.K2_ActivateAbility`
  (bind _returnvalue (`self.GetAvatarActorFromActorInfo`))
  (`self.K2_CommitAbility`)
  (`AbilityTask_PlayMontageAndWait.CreatePlayMontageAndWaitProxy` "None" (`self.Montage to Play`)
    (:`then`
      (`AbilityTask_WaitGameplayEvent.WaitGameplayEvent` (struct :`TagName` "Event.ComboWindowOpen") null
        (:`then`
          (`AbilityTask_WaitGameplayEvent.WaitGameplayEvent` (struct :`TagName` "Event.ComboWindowClose") null
            (:`EventReceived`
              (`AbilitySystemBlueprintLibrary.RemoveLooseGameplayTags` (`self.GetAvatarActorFromActorInfo`) (`self.ComboWindowOpenTag`))
              (`self.K2_EndAbility`))))
        (:`EventReceived`
          (`AbilitySystemBlueprintLibrary.RemoveLooseGameplayTags` _returnvalue (`self.ComboWindowOpenTag_Previes`))
          (`AbilitySystemBlueprintLibrary.AddLooseGameplayTags` _returnvalue (`self.ComboWindowOpenTag`)))))
    (:`OnCompleted`
      (`self.K2_EndAbility`))))