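; Gameplay Ability that deals instant area damage around its owner.
; On activation it sphere-overlaps Pawn objects within Radius of the owner's location and draws a red debug sphere of the same size.
; The owner's Ability System Component applies GE_SimpleDamage to each overlapped actor's component, with no ignore list or team filter, then the ability ends.
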(event `self.K2_ActivateAbility`
  (bind _radius (`self.Radius`))
  (bind ((`OwnerActor` _owneractor)) (break `GameplayAbilityActorInfo` (`self.GetActorInfo`)))
  (bind _returnvalue (`Actor.K2_GetActorLocation` _owneractor))
  (`KismetSystemLibrary.DrawDebugSphere` _returnvalue _radius 12 (struct :`R` 1.0 :`A` 1.0) 1.0 10.0)
  (bind (_outactors _returnvalue_2) (`KismetSystemLibrary.SphereOverlapActors` _returnvalue _radius (`|MakeArray` "ObjectTypeQuery3" :!type "EObjectTypeQuery Enum")))
  (if _returnvalue_2
    (for _array_element _outactors
      (`AbilitySystemComponent.BP_ApplyGameplayEffectToTarget` :`self` (`AbilitySystemBlueprintLibrary.GetAbilitySystemComponent` _owneractor) :`GameplayEffectClass` "/Game/GAS/Effects/GE_SimpleDamage.GE_SimpleDamage_C" :`Target` (`AbilitySystemBlueprintLibrary.GetAbilitySystemComponent` _array_element) :`Level` 1.0)))
  (`self.K2_EndAbility`))