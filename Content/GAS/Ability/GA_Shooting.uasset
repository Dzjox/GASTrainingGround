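; GA_Shooting is a Gameplay Ability that fires arrows repeatedly while the input is held.
; After committing, it shoots immediately and starts a looping timer whose rate comes from an attribute on the avatar, ending on input release.
; Each shot gets muzzle location and aim rotation through avatar messages, then spawns BP_Arrow with the instigator ASC, a GE_DamageWithArmor spec and damage scaled by ability level.
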(event `self.K2_ActivateAbility`
  (bind (_bsuccessfullyfoundattribute _returnvalue) (`AbilitySystemBlueprintLibrary.GetFloatAttribute` (`self.GetAvatarActorFromActorInfo`) (struct :`AttributeName` "AttackSpeed" :`Attribute` "/Script/GASTrainingGround.AttributeSetBase:AttackSpeed" :`AttributeOwner` "/Script/CoreUObject.Class'/Script/GASTrainingGround.AttributeSetBase'")))
  (bind _returnvalue_2 (`self.K2_CommitAbility`))
  (if _returnvalue_2
    (if _bsuccessfullyfoundattribute
      (`KismetSystemLibrary.K2_SetTimerDelegate` (delegate `Shooting`) (/ 1.0 _returnvalue) true)
      (`self.Shooting`)
      (`AbilityTask_WaitInputRelease.WaitInputRelease` false
        (:`OnRelease`
          (`self.K2_EndAbility`)))
      (else
        (`self.K2_EndAbility`)))
    (else
      (`self.K2_EndAbility`))))

(event `Shooting`
  (bind _returnvalue (`self.GetAvatarActorFromActorInfo`))
  (bind _returnvalue_2 (`AbilitySystemBlueprintLibrary.GetAbilitySystemComponent` _returnvalue))
  (bind (_location _relevant) (message `/Game/GAS/Interfaces/I_Crossbow.GetMuzzleLocation` (`self.GetAvatarActorFromActorInfo`)))
  (if _relevant
    (bind _rotation (message `/Game/GAS/Interfaces/I_Crossbow.GetShootingRotation` _returnvalue))
    (`|SpawnActorFromClass` "/Game/GAS/Blueprints/BP_Arrow.BP_Arrow_C" (`KismetMathLibrary.MakeTransform` _location _rotation) "Undefined" "MultiplyWithRoot" null _returnvalue_2 (`AbilitySystemComponent.MakeOutgoingSpec` :`self` _returnvalue_2 :`GameplayEffectClass` "/Game/GAS/Effects/GE_DamageWithArmor.GE_DamageWithArmor_C") (+ (* (`KismetMathLibrary.Conv_IntToDouble` (`self.GetAbilityLevel`)) (`self.DamagePerLevel`)) (`self.Damage`)) null)
    (else
      (`self.K2_EndAbility`))))