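; GA_Fireball is a Gameplay Ability that launches a BP_Fireball projectile from the avatar's muzzle.
; After committing, it gets muzzle location and shooting rotation through messages to the avatar, spawning only if the location is relevant.
; The projectile receives a sphere radius and a GE_DamageWithArmor spec at ability level, with damage set by caller through the Data.Damage tag.
; The ability ends immediately on every path.
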(event `self.K2_ActivateAbility`
  (bind _returnvalue (`self.GetAvatarActorFromActorInfo`))
  (bind _returnvalue_2 (`self.K2_CommitAbility`))
  (if _returnvalue_2
    (bind (_location _relevant) (message `/Game/GAS/Interfaces/I_Crossbow.GetMuzzleLocation` (`self.GetAvatarActorFromActorInfo`)))
    (if _relevant
      (bind _rotation (message `/Game/GAS/Interfaces/I_Crossbow.GetShootingRotation` _returnvalue))
      (bind _returnvalue_3 (`AbilitySystemBlueprintLibrary.AssignTagSetByCallerMagnitude` (`AbilitySystemComponent.MakeOutgoingSpec` :`self` (`AbilitySystemBlueprintLibrary.GetAbilitySystemComponent` _returnvalue) :`GameplayEffectClass` "/Game/GAS/Effects/GE_DamageWithArmor.GE_DamageWithArmor_C" :`Level` (`KismetMathLibrary.Conv_IntToDouble` (`self.GetAbilityLevel`))) (struct :`TagName` "Data.Damage") (`self.Damage`)))
      (`|SpawnActorFromClass` "/Game/GAS/Blueprints/BP_Fireball.BP_Fireball_C" (`KismetMathLibrary.MakeTransform` _location _rotation) "Undefined" "MultiplyWithRoot" null null _returnvalue_3 (`self.Sphere Radius`) (cast `Pawn` _returnvalue :!pure true))
      (`self.K2_EndAbility`)
      (else
        (`self.K2_EndAbility`)))
    (else
      (`self.K2_EndAbility`))))