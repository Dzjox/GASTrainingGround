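; GAS-driven enemy that chases the player and attacks guards with a mutant attack ability.
; Attribute data sets health, armor, speed and scale through SetByCaller effects and direct setters, while a looping timer restarts stalled movement.
; Capsule hits activate the attack; spike overlaps send its gameplay event.
; Damage routes through effects mapped to armor components; attribute changes spawn floating damage and trigger one-time ragdoll death with delayed destruction.
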(event `self.ReceiveBeginPlay`
  (`|ExecutionSequence`
    (:`then_0`
      (bind _asw_health_bar (cast `/Game/HUD/W_HealthBar` (`WidgetComponent.GetWidget` (`self.HPBar`))))
      (set `/Game/HUD/W_HealthBar.AbilitySystemComponent` (`self.AbilitySystem`) _asw_health_bar))
    (:`then_1`
      (bind (_asynctaskproxy _attribute _newvalue _oldvalue) (`AbilityAsync_WaitAttributeChanged.WaitForAttributeChanged` null (struct :`AttributeName` "Health" :`Attribute` "/Script/GASTrainingGround.AttributeSetBase:Health" :`AttributeOwner` "/Script/CoreUObject.Class'/Script/GASTrainingGround.AttributeSetBase'"))
        (:`Changed`
          (`self.SpwanDamageWidget` (- _newvalue _oldvalue))
          (if (<= _newvalue 0.0)
            (`/Engine/EditorBlueprintResources/StandardMacros.DoOnce` false
              (:`Completed`
                (`self.DIE!`)))))))
    (:`then_2`
      (bind _returnvalue (`KismetSystemLibrary.K2_SetTimerDelegate` (`|CreateDelegate` :!event `TryReinitMovement`) 1.0 true))
      (set `self.TryReinitMovementTimer` _returnvalue)
      (`self.ApplyAttributes`)
      (`AbilitySystemComponent.K2_GiveAbility` (`self.AbilitySystem`) "/Game/GAS/Ability/GA_MutantAttack.GA_MutantAttack_C" 0 -1))))

(event `self.CapsuleComponent.OnComponentHit`
  (params (HitComponent :type "PrimitiveComponent Object Reference") (OtherActor :type "Actor Object Reference") (OtherComp :type "PrimitiveComponent Object Reference") (NormalImpulse :type "Vector Structure") (Hit :type "HitResult Structure (by ref)"))
  (cast `/Game/GAS/Blueprints/BP_Guard` OtherActor)
  (`AbilitySystemComponent.TryActivateAbilitiesByTag` (`self.AbilitySystem`) (`BlueprintGameplayTagLibrary.MakeLiteralGameplayTagContainer` (struct :`GameplayTags` (struct :`(TagName` "Ability.MutanAttack")))) true))

(event `TryReinitMovement`
  (if (== (`self.GetVelocity`) (0.0 0.0 0.0) :`ErrorTolerance` 10.0)
    (bind _asaicontroller (cast `AIController` (`self.GetController`)))
    (`AIController.MoveToActor` _asaicontroller (`self.Player`) -1.0 false true true null true)))

(event `DIE!`
  (bind _mesh (`self.Mesh`))
  (`PrimitiveComponent.SetSimulatePhysics` _mesh true)
  (`PrimitiveComponent.SetCollisionProfileName` _mesh "Ragdoll" true)
  (`AbilitySystemBlueprintLibrary.AddLooseGameplayTags` self (`self.DeadTags`))
  (`SceneComponent.SetHiddenInGame` (`self.HPBar`) true false)
  (`self.OnDeath` self)
  (`KismetSystemLibrary.K2_ClearAndInvalidateTimerHandle` (`self.TryReinitMovementTimer`))
  (`MovementComponent.StopMovementImmediately` (`self.CharacterMovement`))
  (`PrimitiveComponent.SetCollisionProfileName` (`self.CapsuleComponent`) "NoCollision" false)
  (`KismetSystemLibrary.Delay` 10.0)
  (`self.K2_DestroyActor`))

(event `ApplyAttributes`
  (bind ((`Scale_15_E206EF78444EEF911A5E2D9958D344F8` _scale)) (break `/Game/GAS/Data/S_EnemyAttributes` (`self.Attributes`)))
  (`|ExecutionSequence`
    (:`then_0`
      (bind _returnvalue (`AbilitySystemBlueprintLibrary.AssignTagSetByCallerMagnitude` (`AbilitySystemComponent.MakeOutgoingSpec` :`self` (`self.AbilitySystem`) :`GameplayEffectClass` "/Game/GAS/Effects/GE_ChangeMaxHealth.GE_ChangeMaxHealth_C") (struct :`TagName` "Data.Attribute") (`KismetMathLibrary.Conv_IntToDouble` (`.Heath_10_C170B00741A146510CD74D833D7CE1A5` (break `/Game/GAS/Data/S_EnemyAttributes` (`self.Attributes`))))))
      (`AbilitySystemComponent.BP_ApplyGameplayEffectSpecToSelf` (`self.AbilitySystem`) _returnvalue))
    (:`then_1`
      (bind _returnvalue_2 (`AbilitySystemBlueprintLibrary.AssignTagSetByCallerMagnitude` (`AbilitySystemComponent.MakeOutgoingSpec` :`self` (`self.AbilitySystem`) :`GameplayEffectClass` "/Game/GAS/Effects/GE_ChangeHealth.GE_ChangeHealth_C") (struct :`TagName` "Data.Attribute") (`KismetMathLibrary.Conv_IntToDouble` (`.Heath_10_C170B00741A146510CD74D833D7CE1A5` (break `/Game/GAS/Data/S_EnemyAttributes` (`self.Attributes`))))))
      (`AbilitySystemComponent.BP_ApplyGameplayEffectSpecToSelf` (`self.AbilitySystem`) _returnvalue_2))
    (:`then_2`
      (bind _returnvalue_3 (`AbilitySystemBlueprintLibrary.AssignTagSetByCallerMagnitude` (`AbilitySystemComponent.MakeOutgoingSpec` :`self` (`self.AbilitySystem`) :`GameplayEffectClass` "/Game/GAS/Effects/GE_ChangeArmor.GE_ChangeArmor_C") (struct :`TagName` "Data.Attribute") (`KismetMathLibrary.Conv_IntToDouble` (`.Armor_11_D281F9B14997EBBFD67F1E859EE4E293` (break `/Game/GAS/Data/S_EnemyAttributes` (`self.Attributes`))))))
      (`AbilitySystemComponent.BP_ApplyGameplayEffectSpecToSelf` (`self.AbilitySystem`) _returnvalue_3))
    (:`then_3`
      (set `CharacterMovementComponent.MaxWalkSpeed` (`KismetMathLibrary.Conv_IntToDouble` (`.Speed_12_A2BD22AD44188D484FF891B2D011F53E` (break `/Game/GAS/Data/S_EnemyAttributes` (`self.Attributes`)))) (`self.CharacterMovement`)))
    (:`then_4`
      (`SceneComponent.SetWorldScale3D` (`self.CapsuleComponent`) (`KismetMathLibrary.MakeVector` _scale _scale _scale)))))

(event `self.SpikeCollision.OnComponentBeginOverlap`
  (params (OverlappedComponent :type "PrimitiveComponent Object Reference") (OtherActor :type "Actor Object Reference") (OtherComp :type "PrimitiveComponent Object Reference") (OtherBodyIndex :type Integer) (bFromSweep :type Boolean) (SweepResult :type "HitResult Structure (by ref)"))
  (bind _asbp_guard (cast `/Game/GAS/Blueprints/BP_Guard` OtherActor))
  (`AbilitySystemBlueprintLibrary.SendGameplayEventToActor` self (struct :`TagName` "Event.MutantAttack") (make `GameplayEventData` (struct :`TagName` "Event.MutantAttack") self _asbp_guard)))

(event `/Game/GAS/Interfaces/I_PlateArmor.ReceiveDamage`
  (params (Damage :type "Float (double-precision)") (ArmorComponents :type "Array of /Game/GAS/Blueprints/BP_PlateArmorComponent Object Reference (by ref)"))
  (for _array_element ArmorComponents
    (bind (_value _returnvalue) (`BlueprintMapLibrary.Map_Find` (`self.ArmorToEffect`) _array_element))
    (if _returnvalue
      (bind _returnvalue_2 (`AbilitySystemBlueprintLibrary.AssignTagSetByCallerMagnitude` (`AbilitySystemComponent.MakeOutgoingSpec` :`self` (`self.AbilitySystem`) :`GameplayEffectClass` _value) (struct :`TagName` "Data.Damage") (- 0.0 Damage)))
      (`AbilitySystemComponent.BP_ApplyGameplayEffectSpecToSelf` (`self.AbilitySystem`) _returnvalue_2))))

(event `/Game/GAS/Interfaces/I_PlateArmor.RemoveArmorComponent`
  (params (Armor :type "/Game/GAS/Blueprints/BP_PlateArmorComponent Object Reference"))
  (`BlueprintMapLibrary.Map_Remove` (`self.ArmorToEffect`) Armor))

(fn `AddArmorComponent`
  (params (NewArmor :type "/Game/GAS/Blueprints/BP_PlateArmorComponent Object Reference"))
  (returns (Attribute :type "GameplayAttribute Structure"))
  (bind _armortoeffect (`self.ArmorToEffect`))
  (bind _keys (`BlueprintMapLibrary.Map_Keys` _armortoeffect))
  (bind _output (`|GetArrayItem` (`self.PlateArmorEffects`) (`KismetArrayLibrary.Array_Length` _keys)))
  (`BlueprintMapLibrary.Map_Add` _armortoeffect NewArmor _output)
  (return (`BlueprintFunctionLibraryMix.GetAttributeFromEffect` _output)))

(fn `SpwanDamageWidget`
  (params (Damage :type "Float (double-precision)"))
  (bind _returnvalue_location (`KismetMathLibrary.BreakTransform` (`self.GetTransform`)))
  (if (not (>= Damage 0.0))
    (bind _returnvalue (`|SpawnActorFromClass` "/Game/GAS/Blueprints/BP_FloatingDamage.BP_FloatingDamage_C" (`KismetMathLibrary.MakeTransform` _returnvalue_location (struct :`Pitch` 90.0)) "Undefined" "MultiplyWithRoot" null Damage null))
    (set `ProjectileMovementComponent.InitialSpeed` 5000.0 (`/Game/GAS/Blueprints/BP_FloatingDamage.ProjectileMovement` _returnvalue))
    (`self.SetLifeSpan` _returnvalue 2.0)))

(fn `UserConstructionScript`)