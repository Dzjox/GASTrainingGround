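; Arena game mode that runs endless, escalating enemy waves against registered guards and levels the guards up from kills.
; Adding a guard starts a looping round timer, which spawns capped batches of BP_Enemy, then raises the next count and attributes.
; Spawn points lie at random angles around the first guard, lifted by repeated upward traces until unobstructed.
; Enemy deaths feed a rising kill threshold that applies GE_LevelUp to every guard through GAS.
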(event `TryStartGame`
  (if (not (`KismetSystemLibrary.K2_IsValidTimerHandle` (`self.RoundTimer`)))
    (set `self.CurrentKillNeedToLevelUp` (`self.StartKillNeedToLevelUp`))
    (set `self.CurrentCount` (`self.StartCount`))
    (set `self.CurrentEnemyAtrributes` (`self.StartEnemyAtrributes`))
    (`KismetSystemLibrary.Delay` 2.0)
    (`self.StartGame`)))

(event `StartGame`
  (bind _returnvalue (`KismetSystemLibrary.K2_SetTimerDelegate` (delegate `StartRound`) (`self.RaundsDelay`) true))
  (set `self.RoundTimer` _returnvalue))

(event `StartRound`
  (`self.SpawnEneny` (`self.CurrentCount`) (`self.CurrentEnemyAtrributes`))
  (`self.UpgradeEnemy`))

(event `SpawnEneny`
  (params (Count :type Integer) (EnemyAttributes :type "/Game/GAS/Data/S_EnemyAttributes Structure"))
  (for _ (range (+ (`KismetMathLibrary.Min` Count (- (`self.MaxEnemies`) (`KismetArrayLibrary.Array_Length` (`self.Enemies`)))) 1))
    (bind _returnvalue (`|SpawnActorFromClass` "/Game/GAS/Blueprints/BP_Enemy.BP_Enemy_C" (`KismetMathLibrary.MakeTransform` (`self.GetPlaceForSpawn`)) "AlwaysSpawn" "MultiplyWithRoot" null EnemyAttributes null))
    (`KismetArrayLibrary.Array_Add` (`self.Enemies`) _returnvalue)
    (add `/Game/GAS/Blueprints/BP_Enemy.OnDeath` _returnvalue (delegate `OnEnemyDead`))))

(event `OnEnemyDead`
  (params (Enemy :type "/Game/GAS/Blueprints/BP_Enemy Object Reference"))
  (`KismetArrayLibrary.Array_RemoveItem` (`self.Enemies`) Enemy)
  (`self.TryLevelUp`))

(event `UpgradeEnemy`
  (bind (_deltatenemyatrributes_heath _deltatenemyatrributes_armor _deltatenemyatrributes_speed _deltatenemyatrributes_scale) (break `/Game/GAS/Data/S_EnemyAttributes` (`self.DeltatEnemyAtrributes`)))
  (bind (_currentenemyatrributes_heath _currentenemyatrributes_armor _currentenemyatrributes_speed _currentenemyatrributes_scale) (break `/Game/GAS/Data/S_EnemyAttributes` (`self.CurrentEnemyAtrributes`)))
  (`|ExecutionSequence`
    (:`then_0`
      (bind _result (`/Engine/EditorBlueprintResources/StandardMacros.IncrementInt` (`self.CurrentCount`))
        (:`  `
          (set `self.StartCount` _result))))
    (:`then_1`
      (set `self.CurrentEnemyAtrributes` (make `/Game/GAS/Data/S_EnemyAttributes` (+ _currentenemyatrributes_heath _deltatenemyatrributes_heath) (+ _currentenemyatrributes_armor _deltatenemyatrributes_armor) (+ _currentenemyatrributes_speed _deltatenemyatrributes_speed) (+ _currentenemyatrributes_scale _deltatenemyatrributes_scale))))))

(event `TryLevelUp`
  (bind _result (`/Engine/EditorBlueprintResources/StandardMacros.IncrementInt` (`self.CurrentKills`))
    (:`  `
      (if (>= _result (`self.CurrentKillNeedToLevelUp`))
        (`/Engine/EditorBlueprintResources/StandardMacros.IncrementInt` (`self.CurrentKillNeedToLevelUp`)
          (:`  `
            (set `self.CurrentKills` 0)
            (for _array_element (`self.Gurds`)
              (`AbilitySystemComponent.BP_ApplyGameplayEffectToSelf` :`self` (`AbilitySystemBlueprintLibrary.GetAbilitySystemComponent` _array_element) :`GameplayEffectClass` "/Game/GAS/Effects/GE_LevelUp.GE_LevelUp_C"))))))))

(fn `AddGuard`
  (params (Guard :type "/Game/GAS/Blueprints/BP_Guard Object Reference (by ref)"))
  (`KismetArrayLibrary.Array_Add` (`self.Gurds`) Guard)
  (`self.TryStartGame`))

(fn `GetPlaceForSpawn`
  (returns (ValidLocation :type "Vector Structure"))
  (locals (SupposeLocation :type "Vector Structure"))
  (bind _supposelocation (`local.SupposeLocation`))
  (set `local.SupposeLocation` (+ (`self.K2_GetActorLocation` (`|GetArrayItem` (`self.Gurds`))) (* (`KismetMathLibrary.GreaterGreater_VectorRotator` (`KismetMathLibrary.MakeVector` 1.0) (`KismetMathLibrary.MakeRotator` 0.0 0.0 (`KismetMathLibrary.RandomFloatInRange` 0.0 360.0))) (`self.SpawnDistance`))))
  (bind (_outhit _returnvalue) (`KismetSystemLibrary.LineTraceSingle` _supposelocation (+ _supposelocation (0.0 0.0 10000.0)) "TraceTypeQuery1" :!label _label))
  (if _returnvalue
    (set `local.SupposeLocation` (+ (`.Location` (`GameplayStatics.BreakHitResult` _outhit)) (0.0 0.0 1000.0)))
    (goto _label)
    (else
      (return (`local.SupposeLocation`)))))

(fn `UserConstructionScript`)