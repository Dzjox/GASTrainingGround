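; BP_ToxicCloud is a toxic area hazard that applies the GE_Toxic gameplay effect to actors with an Ability System Component inside its Box.
; Box overlap events add and remove those components in an array.
; Tick loops over the array and applies the effect at a fixed level every frame, so the application rate follows the tick rate.
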(event `self.Box.OnComponentBeginOverlap`
  (params (OverlappedComponent :type "PrimitiveComponent Object Reference") (OtherActor :type "Actor Object Reference") (OtherComp :type "PrimitiveComponent Object Reference") (OtherBodyIndex :type Integer) (bFromSweep :type Boolean) (SweepResult :type "HitResult Structure (by ref)"))
  (bind _returnvalue (`AbilitySystemBlueprintLibrary.GetAbilitySystemComponent` OtherActor))
  (`/Engine/EditorBlueprintResources/StandardMacros.IsValid` _returnvalue
    (:`Is Valid`
      (`KismetArrayLibrary.Array_Add` (`self.AbilitySystemComponents`) _returnvalue))))

(event `self.Box.OnComponentEndOverlap`
  (params (OverlappedComponent :type "PrimitiveComponent Object Reference") (OtherActor :type "Actor Object Reference") (OtherComp :type "PrimitiveComponent Object Reference") (OtherBodyIndex :type Integer))
  (bind _returnvalue (`AbilitySystemBlueprintLibrary.GetAbilitySystemComponent` OtherActor))
  (`/Engine/EditorBlueprintResources/StandardMacros.IsValid` _returnvalue
    (:`Is Valid`
      (`KismetArrayLibrary.Array_RemoveItem` (`self.AbilitySystemComponents`) _returnvalue))))

(event `self.ReceiveTick`
  (params (DeltaSeconds :type "Float (single-precision)"))
  (for _array_element (`self.AbilitySystemComponents`)
    (`AbilitySystemComponent.BP_ApplyGameplayEffectToSelf` :`self` _array_element :`GameplayEffectClass` "/Game/GAS/Effects/GE_Toxic.GE_Toxic_C" :`Level` 1.0)))

(fn `UserConstructionScript`)