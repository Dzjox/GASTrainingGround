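; Fireball projectile actor that explodes when its sphere hits anything but the instigator, dealing area damage to overlapped pawn components.
; Each component whose owner has an ability system gets the damage effect spec from the instigator's ASC, with magnitude set by caller.
; Owners tagged as plate-armored instead receive a damage message, sent only for overlapped plate armor components.
; It then spawns a Niagara explosion and destroys itself.
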(event `self.Sphere.OnComponentHit`
  (params (HitComponent :type "PrimitiveComponent Object Reference") (OtherActor :type "Actor Object Reference") (OtherComp :type "PrimitiveComponent Object Reference") (NormalImpulse :type "Vector Structure") (Hit :type "HitResult Structure (by ref)"))
  (if (not (== OtherActor (`self.GetInstigator`)))
    (`|ExecutionSequence`
      (:`then_0`
        (bind _outcomponents (`KismetSystemLibrary.SphereOverlapComponents` (`self.K2_GetActorLocation`) (`self.Sphere Radius`) (`|MakeArray` "ObjectTypeQuery3" :!type "EObjectTypeQuery Enum")))
        (for _array_element _outcomponents
          (bind _output_get (set `self.TargetComponent` _array_element))
          (bind _returnvalue (`AbilitySystemBlueprintLibrary.GetAbilitySystemComponent` (`ActorComponent.GetOwner` _output_get)))
          (`/Engine/EditorBlueprintResources/StandardMacros.IsValid` _returnvalue
            (:`Is Valid`
              (bind _output_get_2 (set `self.TargetASC` _returnvalue))
              (if (not (`GameplayTagAssetInterface.HasMatchingGameplayTag` _output_get_2 (struct :`TagName` "Condition.HasPlateArmor")))
                (bind _returnvalue_2 (`AbilitySystemBlueprintLibrary.AssignTagSetByCallerMagnitude` (`self.Spec Handle`) (struct :`TagName` "Data.Damage") (`self.Damage`)))
                (`AbilitySystemComponent.BP_ApplyGameplayEffectSpecToTarget` (`AbilitySystemBlueprintLibrary.GetAbilitySystemComponent` (`self.GetInstigator`)) _returnvalue_2 (`self.TargetASC`))
                (else
                  (bind _asbp_plate_armor_component (cast `/Game/GAS/Blueprints/BP_PlateArmorComponent` (`self.TargetComponent`)))
                  (message `/Game/GAS/Interfaces/I_PlateArmor.ReceiveDamage` (`ActorComponent.GetOwner` (`self.TargetASC`)) (`self.Damage`) (`|MakeArray` _asbp_plate_armor_component))))))))
      (:`then_1`
        (`NiagaraFunctionLibrary.SpawnSystemAtLocation` "/Game/GAS/Niagara/NSA_Explosion.NSA_Explosion" (`self.K2_GetActorLocation`) (`self.K2_GetActorRotation`))
        (`self.K2_DestroyActor`)))))

(fn `UserConstructionScript`)