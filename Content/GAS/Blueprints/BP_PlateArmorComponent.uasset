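; Plate armor mesh component for GAS actors that acts as a breakable armor piece with flash feedback.
; On BeginPlay it adds a plate armor tag to the owner, registers through an owner message that returns the attribute to watch, and creates a dynamic material.
; Attribute changes trigger an emissive hit flash that fades by timer, with a separate color for protect flashes.
; At zero it removes the tag, detaches with physics, then unregisters and destroys itself after a delay.
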(event `self.ReceiveBeginPlay`
  (`/Engine/EditorBlueprintResources/StandardMacros.IsValid` (`AbilitySystemBlueprintLibrary.GetAbilitySystemComponent` (`self.GetOwner`))
    (:`Is Valid`
      (`|ExecutionSequence`
        (:`then_0`
          (`AbilitySystemBlueprintLibrary.AddLooseGameplayTags` (`self.GetOwner`) (`self.PlateArmorTag`) true)
          (bind _attribute (message `/Game/GAS/Interfaces/I_PlateArmor.AddArmorComponent` (`self.GetOwner`) self))
          (set `self.Attribute` _attribute)
          (bind _returnvalue (`self.CreateDynamicMaterialInstance` 0 (`self.GetMaterial` 0)))
          (set `self.MainMaterial` _returnvalue))
        (:`then_1`
          (bind (_asynctaskproxy _attribute_2 _newvalue) (`AbilityAsync_WaitAttributeChanged.WaitForAttributeChanged` (`self.GetOwner`) (`self.Attribute`))
            (:`Changed`
              (`self.HitEmissive`)
              (if (<= _newvalue 0.0)
                (`AbilitySystemBlueprintLibrary.RemoveLooseGameplayTags` (`self.GetOwner`) (`self.PlateArmorTag`))
                (`self.K2_DetachFromComponent` "KeepWorld" "KeepWorld" "KeepWorld")
                (`self.SetSimulatePhysics` true)
                (`KismetSystemLibrary.Delay` 2.0)
                (message `/Game/GAS/Interfaces/I_PlateArmor.RemoveArmorComponent` (`self.GetOwner`) self)
                (`self.K2_DestroyComponent`)))))))))

(event `InitFlash`
  (params (Color :type "Color Structure (by ref)"))
  (bind _mainmaterial (`self.MainMaterial`)
    (:`then`
      (`MaterialInstanceDynamic.SetVectorParameterValue` _mainmaterial "EmissiveFactor" (`KismetMathLibrary.Conv_ColorToLinearColor` Color))
      (`MaterialInstanceDynamic.SetScalarParameterValue` _mainmaterial "EmissiveStrength" 1.0)
      (set `self.EmissiveStrength` 1.0)
      (if (not (`KismetSystemLibrary.K2_IsValidTimerHandle` (`self.FlashTimer`)))
        (bind _returnvalue (`KismetSystemLibrary.K2_SetTimerDelegate` (`|CreateDelegate` :!event `EmissiveFall`) 0.1 true))
        (set `self.FlashTimer` _returnvalue)))
    (:`else`)))

(event `HitEmissive`
  (`self.InitFlash` (`self.HitEmissiveColor`)))

(event `ProtectEmissive`
  (`self.InitFlash` (`self.ProtectEmissiveColor`)))

(event `EmissiveFall`
  (bind _output_get (set `self.EmissiveStrength` (- (`self.EmissiveStrength`) 0.2)))
  (`MaterialInstanceDynamic.SetScalarParameterValue` (`self.MainMaterial`) "EmissiveStrength" _output_get)
  (if (< (`self.EmissiveStrength`) 0.0)
    (`KismetSystemLibrary.K2_ClearAndInvalidateTimerHandle` (`self.FlashTimer`))))